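; Ball character that moves on timed key commands by overwriting CharacterMovement velocity every Tick.
; W, S, A and D set direction flags that expire after two-second delays; most clear the other flags, and H clears all.
; Tick turns flags into velocity along the actor's forward axis, or adds a sideways push to the last velocity.
; CheckInstruction is an empty stub, and Chinese command-string comparisons are left unused.
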(event EventTick
  (params (DeltaSeconds :type Float%20%28single-precision%29))
  (bind _charactermovement (Variables|Character|GetCharacterMovement))
  (bind _charactermovement_2 (Variables|Character|GetCharacterMovement))
  (Utilities|FlowControl|Sequence
    (:then_0
      (if (Variables|Default|GetbForward)
        (Variables|/Script/Engine.MovementComponent|SetVelocity _charactermovement_2 (* (Math|Vector|Normalize (Transformation|GetActorForwardVector)) 8e+02))
        (else
          (if (Variables|Default|GetbBack) :!label _label
            (Variables|/Script/Engine.MovementComponent|SetVelocity _charactermovement_2 (* (Math|Vector|Normalize (Transformation|GetActorForwardVector)) -8e+02))
            (else
              (if (Variables|Default|GetbRight) :!label _label_2
                (Variables|/Script/Engine.MovementComponent|SetVelocity _charactermovement (+ (* (Math|Vector|Normalize (Math|Vector|RotateVectorAroundAxis (Transformation|GetActorForwardVector) 9e+01 "0, 0,1.000000")) 4e+02) (Pawn|Components|CharacterMovement|GetLastUpdateVelocity _charactermovement)))
                (else
                  (if (Variables|Default|GetbLeft) :!label _label_3
                    (Variables|/Script/Engine.MovementComponent|SetVelocity _charactermovement (+ (* (Math|Vector|Normalize (Math|Vector|RotateVectorAroundAxis (Transformation|GetActorForwardVector) -9e+01 "0, 0,1.000000")) 4e+02) (Pawn|Components|CharacterMovement|GetLastUpdateVelocity _charactermovement)))))))))))
    (:then_1
      (goto _label))
    (:then_2
      (goto _label_2))
    (:then_3
      (goto _label_3))))

(event Input|KeyboardEvents|W
  (params (Key :type Key%20Structure :default "None"))
  (:Pressed
    (Variables|Default|SetbBack false)
    (Variables|Default|SetbRight false)
    (Variables|Default|SetbLeft false)
    (Variables|Default|SetbForward true)
    (Utilities|FlowControl|Delay 2.0)
    (Variables|Default|SetbForward false)))

(event Input|KeyboardEvents|H
  (params (Key :type Key%20Structure :default "None"))
  (:Pressed
    (Variables|Default|SetbForward false)
    (Variables|Default|SetbBack false)
    (Variables|Default|SetbRight false)
    (Variables|Default|SetbLeft false)))

(event Input|KeyboardEvents|S
  (params (Key :type Key%20Structure :default "None"))
  (:Pressed
    (Variables|Default|SetbForward false)
    (Variables|Default|SetbRight false)
    (Variables|Default|SetbLeft false)
    (Variables|Default|SetbBack true)
    (Utilities|FlowControl|Delay 2.0)
    (Variables|Default|SetbBack false)))

(event Input|KeyboardEvents|D
  (params (Key :type Key%20Structure :default "None"))
  (:Pressed
    (Variables|Default|SetbForward false)
    (Variables|Default|SetbBack false)
    (Variables|Default|SetbLeft false)
    (Variables|Default|SetbRight true)
    (Utilities|FlowControl|Delay 2.0)
    (Variables|Default|SetbRight false)))

(event Input|KeyboardEvents|A
  (params (Key :type Key%20Structure :default "None"))
  (:Pressed
    (Variables|Default|SetbLeft true)
    (Utilities|FlowControl|Delay 2.0)
    (Variables|Default|SetbLeft false)))

(fn ConstructionScript)

(fn CheckInstruction)